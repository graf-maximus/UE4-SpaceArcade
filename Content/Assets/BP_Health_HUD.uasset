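; Arcade HUD that draws health, score and a pause button, and opens the pause and game-over menus.
; Each frame it draws a column of hearts from the game mode's health component, the points at the top and a clickable pause hit box at top right.
; Helper functions scale by viewport and anchor positions to screen fractions.
; Pause clicks and the game mode's game-over event add their menu widgets and pause the game.
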(event Custom|OnGameOver
  (bind _returnvalue (UserInterface|CreateWidget "/Game/Blueprints/Widgets/GameOverMenu.GameOverMenu_C" (Game|Player|GetOwningPlayerController)))
  (UserInterface|Viewport|AddtoViewport _returnvalue 0)
  (Game|SetGamePaused true))

(event EventDrawHUD
  (params (SizeX :type Integer) (SizeY :type Integer))
  (CallFunction|DrawHealth)
  (CallFunction|DrawPause)
  (CallFunction|DrawPoints))

(event EventHitBoxClick
  (params (BoxName :type Name :default "None"))
  (switch name BoxName
    (:Pause
      (if (not (Game|IsGamePaused))
        (bind _returnvalue (UserInterface|CreateWidget "/Game/Blueprints/Widgets/PauseMenu.PauseMenu_C" (Game|Player|GetOwningPlayerController)))
        (UserInterface|Viewport|AddtoViewport _returnvalue 0)
        (Game|SetGamePaused true)))))

(event EventBeginPlay
  (bind _asarcade_game_mode_base (Utilities|Casting|CastToArcadeGameModeBase (Game|GetGameMode)))
  (EventDispatchers|AssignGameOver _asarcade_game_mode_base (delegate Custom|OnGameOver)))

(fn ConstructionScript)

(fn ScaledCoord
  (params (In :type Vector%202D%20Structure))
  (return (* In (Class|WidgetLayoutLibrary|GetViewportScale))))

(fn DrawHealth
  (bind _out (CallFunction|ScaledCoord "(X=80.000000,Y=80.000000)"))
  (bind _returnvalue (Class|GameHealthComponent|GetHealth (Variables|/Script/Arcade.ArcadeGameModeBase|GetGameHealthComponent (.AsArcade%20Game%20Mode%20Base (Utilities|Casting|CastToArcadeGameModeBase (Game|GetGameMode))))))
  (for _index (range 0 (- _returnvalue 1))
    (Canvas|DrawTexture "/Game/Assets/UI/Heart.Heart" (.x (CallFunction|ScaledCoord (Math|Vector2D|MakeVector2D 14.0 (+ (* _index (+ 8e+01 13.0)) 13.0)))) (.y (CallFunction|ScaledCoord (Math|Vector2D|MakeVector2D 14.0 (+ (* _index (+ 8e+01 13.0)) 13.0)))) (.x _out) (.y _out) 0.0 0.0 1.0 1.0 "(R=1.000000,G=1.000000,B=1.000000,A=1.000000)")))

(fn DrawPause
  (bind _out (CallFunction|ScaledCoord "(X=140.000000,Y=140.000000)"))
  (bind _out_2 (CallFunction|ScaledCoord "(X=-140.000000,Y=0.000000)"))
  (bind _out_3 (CallFunction|Anchor _out_2 "(X=1.000000,Y=0.000000)"))
  (Canvas|DrawTexture "/Game/Assets/UI/Pause.Pause" (.x _out_3) (.y _out_3) (.x _out) (.y _out) 0.0 0.0 1.0 1.0 "(R=1.000000,G=1.000000,B=1.000000,A=1.000000)")
  (Class|HUD|AddHitBox (CallFunction|Anchor (CallFunction|ScaledCoord "(X=-140.000000,Y=0.000000)") "(X=1.000000,Y=0.000000)") (CallFunction|ScaledCoord "(X=140.000000,Y=140.000000)") "Pause" false))

(fn Anchor
  (params (InVec :type Vector%202D%20Structure) (Anchor :type Vector%202D%20Structure))
  (return (+ InVec (* Anchor (Viewport|GetViewportSize)))))

(fn DrawPoints
  (bind _returnvalue (Game|GetGameMode))
  (bind _asarcade_game_mode_base (Utilities|Casting|CastToArcadeGameModeBase _returnvalue))
  (bind _returnvalue_2 (Class|ArcadeGameModeBase|GetPoints _asarcade_game_mode_base))
  (bind _returnvalue_3 (Utilities|String|ToString(Integer) _returnvalue_2))
  (bind _outwidth (Class|HUD|GetTextSize _returnvalue_3 0 1.0))
  (bind _returnvalue_4 (/ _outwidth -0.25))
  (bind _out (CallFunction|ScaledCoord (Math|Vector2D|MakeVector2D _returnvalue_4 2e+01)))
  (bind _out_2 (CallFunction|Anchor _out "(X=0.500000,Y=0.000000)"))
  (HUD|DrawText (Utilities|String|ToString(Integer) _returnvalue_2) "(R=0.916667,G=1.000000,B=0.946306,A=1.000000)" (.x _out_2) (.y _out_2) "/Game/Assets/Fonts/F_BigRoboto.F_BigRoboto" 1.0 false))