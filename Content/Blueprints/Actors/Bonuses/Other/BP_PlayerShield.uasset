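; Player shield bonus actor that shows its remaining active time in an on-screen progress bar.
; BeginPlay creates a ShieldTimeRemaining widget and adds it to the viewport.
; Each Tick sets the bar to the DeactivateTimer's remaining time normalized against DeactivateTime, removing the widget when it is nearly empty.
; The timer is not started in these graphs, and GetShieldTime only returns zero.
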(event EventTick
  (params (DeltaSeconds :type Float%20%28single-precision%29))
  (bind _deactivatetimer (Variables|Default|GetDeactivateTimer))
  (bind _deactivatetime (Variables|Default|GetDeactivateTime))
  (bind _shieldtimeremaining_widget (Variables|Default|GetShieldTimeRemaining%20Widget))
  (bind _returnvalue (Utilities|Time|GetTimerRemainingTimebyHandle _deactivatetimer))
  (bind _p_progressbar (Variables|/Game/Blueprints/Widgets/ShieldTimeRemaining.ShieldTimeRemaining_C|GetP_ProgressBar _shieldtimeremaining_widget))
  (bind _returnvalue_2 (Math|Float|NormalizetoRange _returnvalue 0.0 _deactivatetime))
  (Utilities|IsValid _p_progressbar
    (:Is%20Valid
      (Progress|SetPercent _p_progressbar _returnvalue_2)
      (if (<= _returnvalue_2 0.01)
        (Widget|RemovefromParent (Variables|Default|GetShieldTimeRemaining%20Widget))))))

(event EventBeginPlay
  (bind _returnvalue (UserInterface|CreateWidget "/Game/Blueprints/Widgets/ShieldTimeRemaining.ShieldTimeRemaining_C"))
  (bind _output_get (Variables|Default|SetShieldTimeRemaining%20Widget _returnvalue))
  (UserInterface|Viewport|AddtoViewport _output_get 0))

(fn ConstructionScript)

(fn GetShieldTime
  (return 0.0))