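; Enemy pawn variant that homes in on the first player's pawn while constantly moving forward.
; After the parent Tick runs, it steps a fixed distance along its local X each frame, without delta-time scaling.
; It then yaws toward the player, clamping the look-at yaw difference to MaxRotation in either direction and scaling it by delta seconds for gradual steering.
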(event EventTick
  (params (DeltaSeconds :type Float%20%28single-precision%29))
  (bind _maxrotation (Variables|Default|GetMaxRotation))
  (|CallParentFunction DeltaSeconds)
  (Transformation|AddActorLocalOffset (Math|Vector|MakeVector 8.0 0.0 0.0) false false)
  (Transformation|AddActorLocalRotation (Math|Rotator|MakeRotator 0.0 0.0 (* (Math|Float|Clamp(Float) (.yaw (Math|Rotator|Delta(Rotator) (Math|Rotator|FindLookatRotation (Transformation|GetActorLocation) (Transformation|GetActorLocation (Game|Player|GetPlayerPawn 0))) (Transformation|GetActorRotation))) (* -1 _maxrotation) _maxrotation) (Utilities|Time|GetWorldDeltaSeconds))) false false))

(fn ConstructionScript)